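; BP_CollectibleEXAM is a collectible pickup whose points, good/bad type and cube material come from the DACollectible data.
; On box overlap with BP_ThirdPersonCharacter it adds its points to the character's TotalPoints and destroys itself.
; Good pickups decrement the player's CheckingGOODC counter.
; The level reloads when that counter is zero with too few points, or when a bad pickup leaves the total negative.
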(event `self.Box.OnComponentBeginOverlap`
  (params (OverlappedComponent :type "PrimitiveComponent Object Reference") (OtherActor :type "Actor Object Reference") (OtherComp :type "PrimitiveComponent Object Reference") (OtherBodyIndex :type Integer) (bFromSweep :type Boolean) (SweepResult :type "HitResult Structure (by ref)"))
  (bind _asbp_third_person_character (cast `/Game/ThirdPerson/Blueprints/BP_ThirdPersonCharacter` OtherActor))
  (set `/Game/ThirdPerson/Blueprints/BP_ThirdPersonCharacter.TotalPoints` (+ (`/Game/ThirdPerson/Blueprints/BP_ThirdPersonCharacter.TotalPoints` _asbp_third_person_character) (`/Game/ESAME/CollectiblesEXAM/DataAsset/DA_Collectibles.Points` (`self.DA_Collectible`))) _asbp_third_person_character)
  (bind _asbp_third_person_character_2 (cast `/Game/ThirdPerson/Blueprints/BP_ThirdPersonCharacter` (`GameplayStatics.GetPlayerPawn` 0)))
  (if (`/Game/ESAME/CollectiblesEXAM/DataAsset/DA_Collectibles.IsGood?` (`self.DA_Collectible`))
    (bind _checkinggood_c (`/Game/ThirdPerson/Blueprints/BP_ThirdPersonCharacter.CheckingGOOD_C` _asbp_third_person_character_2))
    (bind _result (`/Engine/EditorBlueprintResources/StandardMacros.DecrementInt` _checkinggood_c)
      (:`  `
        (`KismetSystemLibrary.PrintString` (`KismetStringLibrary.Conv_IntToString` _result))
        (if (and (== _checkinggood_c 0) (< (`/Game/ThirdPerson/Blueprints/BP_ThirdPersonCharacter.TotalPoints` _asbp_third_person_character_2) 2))
          (`/Game/ThirdPerson/Blueprints/BP_ThirdPersonCharacter.ReloadLevel` _asbp_third_person_character :!label _label)
          (`self.K2_DestroyActor`)
          (else
            (`self.K2_DestroyActor`)))))
    (elif (< (`/Game/ThirdPerson/Blueprints/BP_ThirdPersonCharacter.TotalPoints` _asbp_third_person_character_2) 0)
      (goto _label)
      (elif (and (== (`/Game/ThirdPerson/Blueprints/BP_ThirdPersonCharacter.CheckingGOOD_C` _asbp_third_person_character_2) 0) (< (`/Game/ThirdPerson/Blueprints/BP_ThirdPersonCharacter.TotalPoints` _asbp_third_person_character_2) 2))
        (goto _label)
        (else
          (`self.K2_DestroyActor`))))))

(event `self.ReceiveBeginPlay`
  (`PrimitiveComponent.SetMaterial` (`self.Cube`) 0 (`/Game/ESAME/CollectiblesEXAM/DataAsset/DA_Collectibles.Material` (`self.DA_Collectible`))))

(fn `DestroyAll`
  (`self.K2_DestroyActor`))

(fn `UserConstructionScript`)