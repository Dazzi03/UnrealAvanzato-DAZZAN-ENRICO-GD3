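; BP_ButtonEXAM is a timed button that adds to ButtonCounter on the third-person game mode when its sphere collision is overlapped.
; For the player character, it turns on with a green material, then after three seconds restores its material and decrements the counter.
; IsOn blocks retriggering while active.
; The increment precedes the character cast, so other overlapping actors raise the counter without activating or undoing it.
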(event `self.SphereCollision.OnComponentBeginOverlap`
  (params (OverlappedComponent :type "PrimitiveComponent Object Reference") (OtherActor :type "Actor Object Reference") (OtherComp :type "PrimitiveComponent Object Reference") (OtherBodyIndex :type Integer) (bFromSweep :type Boolean) (SweepResult :type "HitResult Structure (by ref)"))
  (if (not (`self.IsOn`))
    (bind _asbp_third_person_game_mode (cast `/Game/ThirdPerson/Blueprints/BP_ThirdPersonGameMode` (`GameplayStatics.GetGameMode`)))
    (`/Engine/EditorBlueprintResources/StandardMacros.IncrementInt` (`/Game/ThirdPerson/Blueprints/BP_ThirdPersonGameMode.ButtonCounter` _asbp_third_person_game_mode)
      (:`  `
        (cast `/Game/ThirdPerson/Blueprints/BP_ThirdPersonCharacter` OtherActor)
        (set `self.IsOn` true)
        (`PrimitiveComponent.SetMaterial` (`self.ButtonMesh`) 0 "/Engine/EngineDebugMaterials/VertexColorViewMode_GreenOnly.VertexColorViewMode_GreenOnly")
        (`KismetSystemLibrary.Delay` 3.0)
        (set `self.IsOn` false)
        (`PrimitiveComponent.SetMaterial` (`self.ButtonMesh`) 0 "/Engine/VREditor/LaserPointer/LaserPointerMaterialInst.LaserPointerMaterialInst")
        (bind _asbp_third_person_game_mode_2 (cast `/Game/ThirdPerson/Blueprints/BP_ThirdPersonGameMode` (`GameplayStatics.GetGameMode`)))
        (`/Engine/EditorBlueprintResources/StandardMacros.DecrementInt` (`/Game/ThirdPerson/Blueprints/BP_ThirdPersonGameMode.ButtonCounter` _asbp_third_person_game_mode_2))))))

(event `self.ReceiveActorBeginOverlap`
  (params (OtherActor :type "Actor Object Reference")))

(fn `UserConstructionScript`)