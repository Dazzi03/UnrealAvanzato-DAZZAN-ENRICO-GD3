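; BP_Door is a door actor that streams in a level and removes itself once trigger and key requirements are met.
; Every Tick it compares the trigger and key counters on BP_ThirdPersonGameMode with its own required quantities, using CheckFirstDoor.
; On a match, NewVar selects Lvl_1 or Lvl_2 to load visibly by soft reference without blocking, and the door then destroys itself.
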(event `self.ReceiveTick`
  (params (DeltaSeconds :type "Float (single-precision)"))
  (bind _asbp_third_person_game_mode (cast `/Game/ThirdPerson/Blueprints/BP_ThirdPersonGameMode` (`GameplayStatics.GetGameMode`)))
  (if (`self.CheckFirstDoor` _asbp_third_person_game_mode _asbp_third_person_game_mode (`self.TriggerQuantity`) (`self.KeyQuantity`))
    (switch `int` (`self.NewVar`)
      (:`0`
        (`GameplayStatics.LoadStreamLevelBySoftObjectPtr` "/Game/ThirdPerson/Lvl_1.Lvl_1" true))
      (:`1`
        (`GameplayStatics.LoadStreamLevelBySoftObjectPtr` "/Game/ThirdPerson/Lvl_2.Lvl_2" true)))
    (`self.K2_DestroyActor`)))

(fn `CheckFirstDoor`
  (params (self2 :type "/Game/ThirdPerson/Blueprints/BP_ThirdPersonGameMode Object Reference") (self3 :type "/Game/ThirdPerson/Blueprints/BP_ThirdPersonGameMode Object Reference") (CounterTriggerBox :type Integer) (CounterKey :type Integer))
  (returns (ReturnValue :type Boolean))
  (return (and (== (`/Game/ThirdPerson/Blueprints/BP_ThirdPersonGameMode.Counter` self3) CounterTriggerBox) (== (`/Game/ThirdPerson/Blueprints/BP_ThirdPersonGameMode.KeyCounter` self2) CounterKey))))

(fn `UserConstructionScript`)