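; Elevator actor that moves its Elevator component between StartingPoint and EndPoint, starting at BeginPlay.
; The CanGoDown flag picks whether the ElevatorMovement timeline plays in reverse or forward, and its track value linearly blends the two world positions.
; On finish, a DoOnce gate leads to a short delay that clears CanGoDown and re-evaluates the direction; nothing here sets the flag true.
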(event `self.ReceiveBeginPlay`
  (`self.StartElevator`))

(event `StartElevator`
  (bind _returnvalue (`SceneComponent.K2_GetComponentLocation` (`self.EndPoint`)))
  (if (`self.CanGoDown`) :!label _label
    (bind (_direction _elevatormovement) (`Timeline|ElevatorMovement` :!via `Reverse` :!label _label_2)
      (:`Update`
        (`SceneComponent.K2_SetWorldLocation` (`self.Elevator`) (+ (* _elevatormovement (- (`SceneComponent.K2_GetComponentLocation` (`self.StartingPoint`)) _returnvalue)) _returnvalue) false false))
      (:`Finished`
        (if (`self.CanGoDown`)
          (goto _label_3 :!via `Reset`)
          (else
            (`/Engine/EditorBlueprintResources/StandardMacros.DoOnce` false :!label _label_3
              (:`Completed`
                (`KismetSystemLibrary.Delay` 2.0)
                (set `self.CanGoDown` false)
                (goto _label)))))))
    (else
      (goto _label_2))))

(fn `UserConstructionScript`)