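; BP_Triggerbox is a one-shot trigger that adds to a shared counter when the third-person character or a projectile overlaps it.
; On overlap it checks the other actor's exact class, then increments Counter on BP_ThirdPersonGameMode and prints the new value.
; A Triggered flag, set after the first successful count, keeps each box from counting again.
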(event `self.ReceiveActorBeginOverlap`
  (params (OtherActor :type "Actor Object Reference"))
  (bind _returnvalue (`GameplayStatics.GetObjectClass` OtherActor))
  (if (or (== _returnvalue "/Game/ThirdPerson/Blueprints/BP_ThirdPersonCharacter.BP_ThirdPersonCharacter_C") (== _returnvalue "/Game/BP_Projectile.BP_Projectile_C"))
    ; Se non ho ancora triggerato
    (if (not (`self.Triggered`))
      (bind _asbp_third_person_game_mode (cast `/Game/ThirdPerson/Blueprints/BP_ThirdPersonGameMode` (`GameplayStatics.GetGameMode`)))
      (bind _output_get (set `/Game/ThirdPerson/Blueprints/BP_ThirdPersonGameMode.Counter` (+ (`/Game/ThirdPerson/Blueprints/BP_ThirdPersonGameMode.Counter` _asbp_third_person_game_mode) 1) _asbp_third_person_game_mode))
      (`KismetSystemLibrary.PrintString` (`KismetStringLibrary.Conv_IntToString` _output_get))
      (set `self.Triggered` true))))

(fn `UserConstructionScript`)